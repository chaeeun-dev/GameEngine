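; Construction-time Blueprint that builds a straight run of static mesh pieces, presumably glass given the asset name, from its origin toward the End vector.
; The Construction Script adds one mesh component every 100 units along the normalized End direction, with the count derived from the vector's length.
; It also moves the Box component one step past the last piece, raised 50 units.
; The event graph holds no runtime logic.
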(event EventBeginPlay)

(event Collision|EventActorBeginOverlap
  (params (OtherActor :type Actor%20Object%20Reference)))

(event EventTick
  (params (DeltaSeconds :type Float%20%28single-precision%29)))

(fn ConstructionScript
  (bind _end (Variables|Default|GetEnd))
  (bind _returnvalue (Math|Vector|VectorLength _end))
  (bind _returnvalue_2 (/ _returnvalue 1e+02))
  (bind _returnvalue_3 (Math|Float|Truncate _returnvalue_2))
  (Variables|Default|SetDirection (Math|Vector|Normalize _end))
  (for _index (range 0 _returnvalue_3)
    (AddComponent|AddStaticMeshComponent false (Math|Conversions|ToTransform(Vector) (* _index 100 (Variables|Default|GetDirection))))
    (Transformation|SetRelativeLocation (Variables|Default|GetBox) (+ (* (+ _returnvalue_3 1) 100 (Variables|Default|GetDirection)) "0.000000,0.000000,50.000000") false false)))