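; BP_Granny is a player-movable pawn driven by the Enhanced Input action IA_MoveGranny.
; Movement input follows the forward and right vectors of the control rotation's yaw only, keeping it horizontal and independent of the actor's facing.
; Each tick, the ControllerDirection component's world rotation is set to the full control rotation.
; An actor-relative version of the movement is left disconnected.
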(event Input|EnhancedActionEvents|EnhancedInputActionIA_MoveGranny
  (params (ActionValue :type Vector%202D%20Structure) (ElapsedSeconds :type Float%20%28double-precision%29) (TriggeredSeconds :type Float%20%28double-precision%29) (InputAction :type Input%20Action%20Object%20Reference :default "/Game/LEC10/IA_MoveGranny.IA_MoveGranny"))
  (bind _returnvalue (Pawn|GetControlRotation :!class /Script/Engine.Pawn))
  (bind _returnvalue_2 (Math|Rotator|MakeRotator 0.0 0.0 (.yaw _returnvalue)))
  (:Triggered
    (Pawn|Input|AddMovementInput (Math|Vector|GetForwardVector _returnvalue_2) (.x ActionValue) false)
    (Pawn|Input|AddMovementInput (Math|Vector|GetRightVector _returnvalue_2) (.y ActionValue) false)))

(event Input|EnhancedActionEvents|EnhancedInputActionIA_MoveGranny
  (params (ActionValue :type Vector%202D%20Structure) (ElapsedSeconds :type Float%20%28double-precision%29) (TriggeredSeconds :type Float%20%28double-precision%29) (InputAction :type Input%20Action%20Object%20Reference :default "/Game/LEC10/IA_MoveGranny.IA_MoveGranny")))

(event EventBeginPlay)

(event Collision|EventActorBeginOverlap
  (params (OtherActor :type Actor%20Object%20Reference)))

(event EventTick
  (params (DeltaSeconds :type Float%20%28single-precision%29))
  (Transformation|SetWorldRotation (Variables|Default|GetControllerDirection) (Pawn|GetControlRotation :!class /Script/Engine.Pawn) false false))

(fn ConstructionScript)